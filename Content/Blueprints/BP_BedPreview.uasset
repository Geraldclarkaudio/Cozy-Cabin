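; Placement preview actor for a bed that shows whether the current spawn spot is valid.
; Parameterless events apply the actor's variables to its StaticMesh, setting collision type, mesh and the first material slot.
; That slot shows a valid or invalid material based on IsValidSpawn, or a default material picked by index from an array.
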(event `SwitchCollisionType`
  (`PrimitiveComponent.SetCollisionEnabled` (`self.StaticMesh`) (`self.CollisionType`)))

(event `SwitchPreviewMesh`
  (`StaticMeshComponent.SetStaticMesh` (`self.StaticMesh`) (`self.newMesh`)))

(event `SwitchMaterial`
  (bind _staticmesh (`self.StaticMesh`))
  (if (`self.isValidSpawn`)
    (`PrimitiveComponent.SetMaterial` _staticmesh 0 (`self.validMaterial`))
    (else
      (`PrimitiveComponent.SetMaterial` _staticmesh 0 (`self.invalidMaterial`)))))

(event `SetDefaultMaterial`
  (`PrimitiveComponent.SetMaterial` (`self.StaticMesh`) 0 (`|GetArrayItem` (`self.DefaultMaterials`) (`self.DefaultMaterialIndex`))))

(fn `UserConstructionScript`)